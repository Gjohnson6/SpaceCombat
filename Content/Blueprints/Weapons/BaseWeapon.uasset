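; Base hitscan weapon actor that damages BaseShip targets, taking its Instigator from the parent Pawn it is attached to.
; ShootWithLoc checks a game-time cooldown, then line-traces from player 0's camera, with Speed scaling the range, to find the aim point.
; A thin sphere trace runs backwards from that point to the supplied start location and applies Damage to any ship hit.
; PlaySoundAtBarrel is a helper not called here.
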(event `self.ReceiveTick`
  (params (DeltaSeconds :type "Float (single-precision)")))

(event `ShootWithLoc`
  (params (StartLocation :type "Vector Structure" :default (0.0 0.0 0.0)))
  ;[1 1 1] Fire
  (bind _canfire (`self.CanFire`))
  (if _canfire
    (`self.UpdateCooldown`)
    (bind _hit_result (`self.TraceCamera`))
    (bind _output_get (set `self.HitLoc` _hit_result))
    (bind _outhit (`KismetSystemLibrary.SphereTraceSingle_NEW` _output_get StartLocation 0.1 "TraceTypeQuery1" false (`|MakeArray` (`self.GetInstigator`) :!type "Actor Object Reference")))
    (bind _asbase_ship (cast `/Game/Blueprints/BaseShip/BaseShip` (`.HitActor` (`GameplayStatics.BreakHitResult` _outhit))))
    (`GameplayStatics.ApplyDamage` _asbase_ship (`self.Damage`) (`GameplayStatics.GetPlayerController` 0) self)))

(fn `CanFire`
  (returns (CanFire :type Boolean))
  (return (<= (`self.Cooldown`) (`KismetSystemLibrary.GetGameTimeInSeconds`))))

(fn `PlaySoundAtBarrel`
  (`GameplayStatics.PlaySoundAtLocation` (`self.Soundclip`) (`SceneComponent.GetSocketLocation` (`self.StaticMesh`) "Barrel")))

(fn `TraceCamera`
  (returns (`Hit Result` :type "Vector Structure") (`Hit Component` :type "ActorComponent Object Reference"))
  (bind _returnvalue (`GameplayStatics.GetPlayerCameraManager` 0))
  (bind _returnvalue_2 (`SceneComponent.K2_GetComponentLocation` (`PlayerCameraManager.TransformComponent` _returnvalue)))
  (bind (_outhit _returnvalue_3) (`KismetSystemLibrary.LineTraceSingle` _returnvalue_2 (+ _returnvalue_2 (* (`self.GetActorForwardVector` _returnvalue) (* (`self.Speed`) 10000.0))) "TraceTypeQuery1" false (`|MakeArray` (`self.GetInstigator`) :!type "Actor Object Reference") "None" true (struct :`R` 0.31152 :`G` 1.0 :`B` 0.065224 :`A` 1.0)))
  (bind (_bblockinghit _binitialoverlap _time _location _impactpoint _normal _impactnormal _physmat _hitactor _hitcomponent _hitbonename _hititem _faceindex _tracestart _traceend) (`GameplayStatics.BreakHitResult` _outhit))
  (return (`KismetMathLibrary.SelectVector` _impactpoint _traceend _returnvalue_3) _hitcomponent))

(fn `UpdateCooldown`
  (set `self.Cooldown` (+ (`self.MaxCooldown`) (`KismetSystemLibrary.GetGameTimeInSeconds`))))

(fn `UserConstructionScript`
  (bind _aspawn (cast `Pawn` (`self.GetParentActor`)))
  (set `self.Instigator` _aspawn))