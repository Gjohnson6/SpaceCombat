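; Test ship pawn Blueprint for trying out axis-driven movement.
; Throttle, right and up axis inputs each feed AddMovementInput along the actor's forward, right and up vectors.
; Tick calls FireWeapons every frame with no input check; that function's body is not in these graphs.
; Controller yaw, pitch and roll calls are present but unwired, so the graph applies no rotation.
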(event `self.ReceiveTick`
  (params (DeltaSeconds :type "Float (single-precision)"))
  (`self.FireWeapons`))

(event `InputAxis|IncreaseThrottle`
  (params (AxisValue :type "Float (single-precision)"))
  (`self.AddMovementInput` (`self.GetActorForwardVector`) AxisValue))

(event `InputAxis|MoveRight`
  (params (AxisValue :type "Float (single-precision)"))
  (`self.AddMovementInput` (`self.GetActorRightVector`) AxisValue))

(event `InputAxis|MoveUp`
  (params (AxisValue :type "Float (single-precision)"))
  (`self.AddMovementInput` (`self.GetActorUpVector`) AxisValue))

(fn `UserConstructionScript`
  (`parent.UserConstructionScript`))