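; PhysShip is a ship Blueprint that appears to be a partly wired physics-based movement experiment.
; Tick eases CurrentSpeed toward DesiredSpeed, then branches on FreeHeld, the momentum input.
; When held, it updates boost lights and speed limits, zeroes boost timers and fires held weapons.
; Otherwise it computes movement values but applies zero force to ShipMesh, while the local-offset move is disconnected.
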(event `self.ReceiveTick`
  (params (DeltaSeconds :type "Float (single-precision)"))
  (bind _basemaxspeed (`self.BaseMaxSpeed`))
  (bind _returnvalue (> (`self.BoostDuration`) 0.0))
  ;[1 1 1] Tick - Move forward/backward
  (bind _output_get (set `self.CurrentSpeed` (`KismetMathLibrary.FInterpTo` (`self.CurrentSpeed`) (`self.DesiredSpeed`) (`GameplayStatics.GetWorldDeltaSeconds`) (/ (`self.AccelerationInterp`) 2.0))))
  ;[1 1 1] Handle momentum when space is held
  (if (`self.FreeHeld`)
    ;[1 1 1] Handle Boost
    (`SceneComponent.SetVisibility` (`self.PointLight4`) _returnvalue false)
    (`SceneComponent.SetVisibility` (`self.PointLight5`) _returnvalue false)
    (set `self.AccelerationInterp` (`KismetMathLibrary.SelectFloat` 0.5 1.0 _returnvalue))
    (set `self.MaxSpeed` (`KismetMathLibrary.SelectFloat` (* _basemaxspeed (`self.BoostMultiplier`)) _basemaxspeed _returnvalue))
    (set `self.BoostDuration` 0.0)
    (set `self.BoostCooldown` 0.0)
    ;[1 1 1] If fire inputs are held, fire the respective weapons
    (if (`self.FireHeld`)
      (`self.FireWeaponType` "NewEnumerator0"))
    (if (`self.SecondaryFireHeld`)
      (`self.FireWeaponType` "NewEnumerator1"))
    (if (`self.MissileFireHeld`)
      (`self.FireWeaponType` "NewEnumerator2"))
    (else
      (bind _output_get_2 (set `self.MovementVector` (`KismetMathLibrary.MakeVector` (+ _output_get 0.0))))
      (set `self.Velocity` (`SceneComponent.GetForwardVector` (`self.ShipMesh`)))
      (`PrimitiveComponent.AddForce` (`self.ShipMesh`) (0.0 0.0 0.0) "None" false))))

(event `InputAction|Free`
  (params (Key :type "Key Structure" :default "AnyKey"))
  (:`Pressed`
    (bind _returnvalue (`PrimitiveComponent.GetPhysicsLinearVelocity` (`self.ShipMesh`) "None"))
    (set `self.Velocity` _returnvalue)))

(fn `UserConstructionScript`
  (`parent.UserConstructionScript`))