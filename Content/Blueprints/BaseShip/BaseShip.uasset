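; Base player-controlled ship with six-axis flight, boost, weapons, health with explosion on destruction, and a front/behind camera toggle.
; Tick interpolates speed toward the throttle-driven target, moves the ship, updates boost timers and fires held weapons.
; Holding Free keeps momentum and unclamps yaw and pitch, and releasing it triggers a boost if off cooldown.
; The construction script assigns weapon child actors, which fire by matching weapon type.
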(event `self.ReceiveTick`
  (params (DeltaSeconds :type "Float (single-precision)"))
  (bind _basemaxspeed (`self.BaseMaxSpeed`))
  (bind (_returnvalue_x _returnvalue_y _returnvalue_z) (`KismetMathLibrary.BreakVector` (`SceneComponent.GetForwardVector` (`self.ShipMesh`))))
  (bind _returnvalue (> (`self.BoostDuration`) 0.0))
  ;[1 1 1] Tick - Move forward/backward
  (bind _output_get (set `self.CurrentSpeed` (`KismetMathLibrary.FInterpTo` (`self.CurrentSpeed`) (`self.DesiredSpeed`) (`GameplayStatics.GetWorldDeltaSeconds`) (/ (`self.AccelerationInterp`) 2.0))))
  ;[1 1 1] Handle momentum when space is held
  (if (`self.FreeHeld`)
    (`self.K2_AddActorWorldOffset` (* (`self.Velocity`) (`KismetMathLibrary.VSize` (`self.MovementVector`))) true)
    (else
      (bind _output_get_2 (set `self.MovementVector` (`KismetMathLibrary.MakeVector` (+ _output_get _returnvalue_x) _returnvalue_y _returnvalue_z)))
      (set `self.Velocity` (`SceneComponent.GetForwardVector` (`self.ShipMesh`)))
      (`self.K2_AddActorLocalOffset` _output_get_2 true)))
  ;[1 1 1] Handle Boost
  (`SceneComponent.SetVisibility` (`self.PointLight4`) _returnvalue false)
  (`SceneComponent.SetVisibility` (`self.PointLight5`) _returnvalue false)
  (set `self.AccelerationInterp` (`KismetMathLibrary.SelectFloat` 0.5 1.0 _returnvalue))
  (set `self.MaxSpeed` (`KismetMathLibrary.SelectFloat` (* _basemaxspeed (`self.BoostMultiplier`)) _basemaxspeed _returnvalue))
  (set `self.BoostDuration` (`self.DecrementByDeltaAndClamp` (`self.BoostDuration`) 0.0 (`self.MaxBoostDuration`)))
  (set `self.BoostCooldown` (`self.DecrementByDeltaAndClamp` (`self.BoostCooldown`) 0.0 (`self.MaxBoostCooldown`)))
  ;[1 1 1] If fire inputs are held, fire the respective weapons
  (`self.FireWeapons`))

(event `InputAxis|IncreaseThrottle`
  (params (AxisValue :type "Float (single-precision)"))
  ;[1 1 1] Throttle
  (if (> AxisValue 0.0)
    (set `self.DesiredSpeed` (`KismetMathLibrary.FInterpTo` (`self.DesiredSpeed`) (`self.MaxSpeed`) (`GameplayStatics.GetWorldDeltaSeconds`) (`self.AccelerationInterp`)))
    (elif (< AxisValue 0.0)
      (set `self.DesiredSpeed` (`KismetMathLibrary.FInterpTo` (`self.DesiredSpeed`) (/ (`self.MaxSpeed`) -2.0) (`GameplayStatics.GetWorldDeltaSeconds`) (`self.AccelerationInterp`))))))

(event `InputAxis|Boost`
  (params (AxisValue :type "Float (single-precision)")))

(event `InputAxis|Yaw`
  (params (AxisValue :type "Float (single-precision)"))
  (bind _maxpitchradiusperframe (`self.MaxPitchRadiusPerFrame`))
  ;[1 1 1] Yaw, Pitch, and Roll
  (if (!= AxisValue 0.0)
    (bind _out (`self.ClampUnless` (`self.FreeHeld`) AxisValue (* _maxpitchradiusperframe -1.0) _maxpitchradiusperframe))
    (`self.K2_AddActorLocalRotation` (`KismetMathLibrary.MakeRotator` 0.0 0.0 _out))))

(event `InputAxis|Pitch`
  (params (AxisValue :type "Float (single-precision)"))
  (bind _maxturnradiusperframe (`self.MaxTurnRadiusPerFrame`))
  ;[1 1 1] Yaw, Pitch, and Roll
  (if (!= AxisValue 0.0)
    (bind _out (`self.ClampUnless` (`self.FreeHeld`) AxisValue (* _maxturnradiusperframe -1.0) _maxturnradiusperframe))
    (`self.K2_AddActorLocalRotation` (`KismetMathLibrary.MakeRotator` 0.0 _out))))

(event `InputAxis|Roll`
  (params (AxisValue :type "Float (single-precision)"))
  ;[1 1 1] Yaw, Pitch, and Roll
  (if (!= AxisValue 0.0)
    (`self.K2_AddActorLocalRotation` (`KismetMathLibrary.MakeRotator` (* AxisValue (`self.RollSpeed`))))))

(event `InputAxis|MoveRight`
  (params (AxisValue :type "Float (single-precision)"))
  ;[1 1 1] Strafing
  (if (!= AxisValue 0.0)
    (`self.K2_AddActorLocalOffset` (`KismetMathLibrary.MakeVector` 0.0 (* (* AxisValue (`self.StrafeSpeed`)) -1.0)) true)))

(event `InputAxis|MoveUp`
  (params (AxisValue :type "Float (single-precision)"))
  ;[1 1 1] Strafing
  (if (!= 0.0 AxisValue)
    (`self.K2_AddActorLocalOffset` (`KismetMathLibrary.MakeVector` 0.0 0.0 (* AxisValue (`self.StrafeSpeed`))) true)))

(event `self.ReceiveDestroyed`
  ;[1 1 1] Handle being destroyed
  (bind _returnvalue (`GameplayStatics.SpawnEmitterAtLocation` "/Game/StarterContent/Particles/P_Explosion.P_Explosion" (`self.K2_GetActorLocation`)))
  (`SceneComponent.SetRelativeScale3D` _returnvalue (5.0 5.0 5.0))
  (`GameplayStatics.SpawnSoundAtLocation` "/Game/StarterContent/Audio/Explosion02.Explosion02"))

(event `self.ReceiveAnyDamage`
  (params (Damage :type "Float (single-precision)") (DamageType :type "DamageType Object Reference") (InstigatedBy :type "Controller Object Reference") (DamageCauser :type "Actor Object Reference"))
  ;[1 1 1] Handle Damage
  (bind _output_get (set `self.Health` (`KismetMathLibrary.FClamp` (- (`self.Health`) Damage) 0.0 (`self.MaxHealth`))))
  (`GameplayStatics.SpawnSoundAtLocation` "/Game/Audio/Heavy_Sci-Fi_Hit_HW_09.Heavy_Sci-Fi_Hit_HW_09" (0.0 0.0 0.0) (struct) 1.0 1.0 0.0 "/Game/HitSoundAttenuation.HitSoundAttenuation")
  (if (<= _output_get 0.0)
    (`self.K2_DestroyActor`)))

(event `InputAction|Fire`
  (params (Key :type "Key Structure" :default "AnyKey"))
  ;[1 1 1] Update whether fire buttons are held
  (:`Pressed`
    (set `self.FireHeld` true))
  (:`Released`
    (set `self.FireHeld` false)))

(event `InputAction|SecondaryFire`
  (params (Key :type "Key Structure" :default "AnyKey"))
  ;[1 1 1] Update whether fire buttons are held
  (:`Pressed`
    (set `self.SecondaryFireHeld` true))
  (:`Released`
    (set `self.SecondaryFireHeld` false)))

(event `InputAction|MissileFire`
  (params (Key :type "Key Structure" :default "AnyKey"))
  ;[1 1 1] Update whether fire buttons are held
  (:`Pressed`
    (set `self.MissileFireHeld` true))
  (:`Released`
    (set `self.MissileFireHeld` false)))

(event `InputAction|Free`
  (params (Key :type "Key Structure" :default "AnyKey"))
  (bind _returnvalue (`KismetMathLibrary.GetRightVector` (struct)))
  (bind _maxspeed (`self.MaxSpeed`))
  (bind _returnvalue_2 (`SceneComponent.K2_GetComponentLocation` (`self.PointLight1`)))
  ;[1 1 1] Update whether free turn button is held
  (:`Pressed`
    (set `self.FreeHeld` true))
  (:`Released`
    (set `self.FreeHeld` false)
    ;[1 1 1] Boost when free turn is released
    (if (<= (`self.BoostCooldown`) 0.0)
      (set `self.DesiredSpeed` _maxspeed)
      (set `self.MaxSpeed` (* _maxspeed (`self.BoostMultiplier`)))
      (set `self.BoostDuration` (`self.MaxBoostDuration`))
      (set `self.BoostCooldown` (`self.MaxBoostCooldown`))
      (`GameplayStatics.SpawnSoundAtLocation` "/Game/Audio/EFX_INT_Siren_Whistle_02.EFX_INT_Siren_Whistle_02" (`SceneComponent.K2_GetComponentLocation` (`self.WaterCollideEngine`)))
      (`SceneComponent.SetVisibility` (`self.PointLight5`) true false)
      (`SceneComponent.SetVisibility` (`self.PointLight4`) true false)
      (`KismetSystemLibrary.DrawDebugCircle` _returnvalue_2 50.0 60 (struct :`G` 0.926059 :`B` 1.0 :`A` 1.0) 3.0 20.0 _returnvalue)
      (`KismetSystemLibrary.DrawDebugCircle` _returnvalue_2 100.0 60 (struct :`G` 0.926059 :`B` 1.0 :`A` 1.0) 3.0 20.0 _returnvalue))))

(event `InputAction|Zoom`
  (params (Key :type "Key Structure" :default "AnyKey"))
  (bind _frontcamera (`self.FrontCamera`))
  (bind _behindcamera (`self.BehindCamera`))
  ;[1 1 1] Toggle Cameras
  (:`Pressed`
    (`/Engine/EditorBlueprintResources/StandardMacros.FlipFlop`
      (:`A`
        (`ActorComponent.SetActive` _frontcamera true false)
        (`ActorComponent.SetActive` _behindcamera false false))
      (:`B`
        (`ActorComponent.SetActive` _behindcamera true false)
        (`ActorComponent.SetActive` _frontcamera false false)))))

(fn `ClampUnless`
  (params (b :type Boolean) (f :type "Float (double-precision)") (lowerBound :type "Float (double-precision)") (upperBound :type "Float (double-precision)"))
  (returns (out :type "Float (double-precision)"))
  (if b
    (return f)
    (else
      (return (`KismetMathLibrary.FClamp` f lowerBound upperBound)))))

(fn `FireWeapons`
  (if (`self.FireHeld`)
    (`self.FireWeaponType` "NewEnumerator0"))
  (if (`self.SecondaryFireHeld`)
    (`self.FireWeaponType` "NewEnumerator1"))
  (if (`self.MissileFireHeld`)
    (`self.FireWeaponType` "NewEnumerator2")))

(fn `FireWeaponType`
  (params (WeaponType :type "/Game/Blueprints/Weapons/WeaponType Enum"))
  (for _array_element (`self.GetAllChildActors` true)
    (bind _asbase_weapon (cast `/Game/Blueprints/Weapons/BaseWeapon` _array_element))
    (if (`|EnumEquality` (`/Game/Blueprints/Weapons/BaseWeapon.WeaponType` _asbase_weapon) WeaponType)
      (`/Game/Blueprints/Weapons/BaseWeapon.ShootWithLoc` _asbase_weapon (0.0 0.0 0.0))))
  (return))

(fn `ResetMaxSpeed`
  (params (Target :type "/Game/Blueprints/BaseShip/BaseShip Object Reference (by ref)"))
  (set `/Game/Blueprints/BaseShip/BaseShip.MaxSpeed` (`/Game/Blueprints/BaseShip/BaseShip.BaseMaxSpeed` Target) Target))

(fn `SlowTo`
  (params (`Target Speed` :type "Float (double-precision)") (Target :type "BaseShipC Object Reference (by ref)"))
  ;[1 1 1] Limit max speed, and if the ship wants to move faster than the new max speed, lower it's desired speed
  (`BaseShipC.SetMaxSpeed` Target `Target Speed`))

(fn `UserConstructionScript`
  (`ChildActorComponent.SetChildActorClass` (`self.Barrel`) "/Game/Blueprints/Weapons/HitscanWeapons/BaseBeam.BaseBeam_C")
  (`ChildActorComponent.SetChildActorClass` (`self.WingLeft`) "/Game/Blueprints/Weapons/ProjectileWeapons/NonHoming/AutoGun.AutoGun_C")
  (`ChildActorComponent.SetChildActorClass` (`self.WingRight`) "/Game/Blueprints/Weapons/ProjectileWeapons/NonHoming/SonarDrill.SonarDrill_C"))