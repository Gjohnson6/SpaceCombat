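; Player-flown spaceship Blueprint with axis-driven rotation and strafing, health, and explosion on death.
; Yaw and pitch are turn-rate clamped unless Free is held; construction assigns weapon child actors.
; Tick just pushes ShipMesh forward at a fixed step.
; Throttle speed, free-flight momentum and primary/secondary firing feed a disconnected chain that never runs; Boost is empty, and Zoom only deactivates cameras.
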(event `self.ReceiveTick`
  (params (DeltaSeconds :type "Float (single-precision)"))
  ;[1 1 1] Tick - Move forward/backward
  (`SceneComponent.K2_AddLocalOffset` (`self.ShipMesh`) (100.0 0.0 0.0) true false))

(event `InputAxis|IncreaseThrottle`
  (params (AxisValue :type "Float (single-precision)"))
  ;[1 1 1] Throttle
  (if (> AxisValue 0.0)
    (set `self.DesiredSpeed` (`KismetMathLibrary.FInterpTo` (`self.DesiredSpeed`) (`self.MaxSpeed`) (`GameplayStatics.GetWorldDeltaSeconds`) (`self.AccelerationInterp`)))
    (elif (< AxisValue 0.0)
      (set `self.DesiredSpeed` (`KismetMathLibrary.FInterpTo` (`self.DesiredSpeed`) (/ (`self.MaxSpeed`) -2.0) (`GameplayStatics.GetWorldDeltaSeconds`) (`self.AccelerationInterp`))))))

(event `InputAxis|Boost`
  (params (AxisValue :type "Float (single-precision)")))

(event `InputAxis|Yaw`
  (params (AxisValue :type "Float (single-precision)"))
  (bind _maxturnradiusperframe (`self.MaxTurnRadiusPerFrame`))
  ;[1 1 1] Yaw, Pitch, and Roll
  (if (!= AxisValue 0.0)
    (bind _ret (`self.ClampUnless` (`self.FreeHeld`) AxisValue (* _maxturnradiusperframe -1.0) _maxturnradiusperframe))
    (`self.K2_AddActorLocalRotation` (`KismetMathLibrary.MakeRotator` 0.0 0.0 (* _ret 0.5)))))

(event `InputAxis|Pitch`
  (params (AxisValue :type "Float (single-precision)"))
  (bind _maxturnradiusperframe (`self.MaxTurnRadiusPerFrame`))
  ;[1 1 1] Yaw, Pitch, and Roll
  (if (!= AxisValue 0.0)
    (bind _ret (`self.ClampUnless` (`self.FreeHeld`) AxisValue (* _maxturnradiusperframe -1.0) _maxturnradiusperframe))
    (`self.K2_AddActorLocalRotation` (`KismetMathLibrary.MakeRotator` 0.0 _ret))))

(event `InputAxis|Roll`
  (params (AxisValue :type "Float (single-precision)"))
  ;[1 1 1] Yaw, Pitch, and Roll
  (if (!= AxisValue 0.0)
    (`self.K2_AddActorLocalRotation` (`KismetMathLibrary.MakeRotator` AxisValue))))

(event `InputAxis|MoveRight`
  (params (AxisValue :type "Float (single-precision)"))
  ;[1 1 1] Strafing
  (if (!= AxisValue 0.0)
    (`self.K2_AddActorLocalOffset` (`KismetMathLibrary.MakeVector` 0.0 (* (* AxisValue (`self.StrafeSpeed`)) -1.0)) true)))

(event `InputAxis|MoveUp`
  (params (AxisValue :type "Float (single-precision)"))
  ;[1 1 1] Strafing
  (if (!= 0.0 AxisValue)
    (`self.K2_AddActorLocalOffset` (`KismetMathLibrary.MakeVector` 0.0 0.0 (* AxisValue (`self.StrafeSpeed`))) true)))

(event `self.ReceiveAnyDamage`
  (params (Damage :type "Float (single-precision)") (DamageType :type "DamageType Object Reference") (InstigatedBy :type "Controller Object Reference") (DamageCauser :type "Actor Object Reference"))
  ;[1 1 1] Handle Damage
  (bind _output_get (set `self.Health` (`KismetMathLibrary.Clamp` (- (`self.Health`) (`KismetMathLibrary.FTrunc` Damage)) 0 (`self.MaxHealth`))))
  (`GameplayStatics.SpawnSoundAtLocation` "/Engine/VREditor/Sounds/VR_negative.VR_negative")
  (if (<= _output_get 0)
    (`self.K2_DestroyActor`)
    (bind _returnvalue (`GameplayStatics.SpawnEmitterAtLocation` "/Game/StarterContent/Particles/P_Explosion.P_Explosion" (`self.K2_GetActorLocation`)))
    (`SceneComponent.SetRelativeScale3D` _returnvalue (5.0 5.0 5.0))
    (`GameplayStatics.SpawnSoundAtLocation` "/Game/StarterContent/Audio/Explosion02.Explosion02")))

(event `InputAction|Fire`
  (params (Key :type "Key Structure" :default "AnyKey"))
  ;[1 1 1] Update whether fire buttons are held
  (:`Pressed`
    (set `self.FireHeld` true))
  (:`Released`
    (set `self.FireHeld` false)))

(event `InputAction|SecondaryFire`
  (params (Key :type "Key Structure" :default "AnyKey"))
  ;[1 1 1] Update whether fire buttons are held
  (:`Pressed`
    (set `self.SecondaryFireHeld` true))
  (:`Released`
    (set `self.SecondaryFireHeld` false)))

(event `InputAction|Free`
  (params (Key :type "Key Structure" :default "AnyKey"))
  ;[1 1 1] Update whether free turn button is held
  (:`Pressed`
    (set `self.FreeHeld` true))
  (:`Released`
    (set `self.FreeHeld` false)))

(event `InputAction|Zoom`
  (params (Key :type "Key Structure" :default "AnyKey"))
  (:`Pressed`
    (`/Engine/EditorBlueprintResources/StandardMacros.FlipFlop`
      (:`A`
        (`ActorComponent.SetActive` (`self.FrontCamera`) false false))
      (:`B`
        (`ActorComponent.SetActive` (`self.BehindCamera`) false false)))))

(fn `ClampUnless`
  (params (b :type Boolean) (f :type "Float (double-precision)") (lowerBound :type "Float (double-precision)") (upperBound :type "Float (double-precision)"))
  (returns (ret :type "Float (double-precision)"))
  (if b
    (return f)
    (else
      (return (`KismetMathLibrary.FClamp` f lowerBound upperBound)))))

(fn `UserConstructionScript`
  (`ChildActorComponent.SetChildActorClass` (`self.Barrel`) "/Game/Blueprints/Weapons/ProjectileWeapons/NonHoming/PlasmaLauncher.PlasmaLauncher_C")
  (`ChildActorComponent.SetChildActorClass` (`self.WingLeft`) null)
  (`ChildActorComponent.SetChildActorClass` (`self.WingRight`) "/Game/Blueprints/Weapons/ProjectileWeapons/NonHoming/AutoGun.AutoGun_C"))