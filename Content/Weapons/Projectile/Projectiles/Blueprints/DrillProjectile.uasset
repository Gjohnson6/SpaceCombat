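; DrillProjectile is a weapon projectile Blueprint whose secondary collision, ActivatedCollision, stays dormant until the projectile hits something.
; The construction script disables that collision, and the Hit event switches it to query-only.
; On actor overlap, it loops over the components overlapping the other actor and calls the parent overlap handler once for each not of object type GameTraceChannel2.
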(event `self.ReceiveActorBeginOverlap`
  (params (OtherActor :type "Actor Object Reference"))
  (for _array_element (`self.GetOverlappingComponents` OtherActor)
    (if (`|EnumInequality` (`PrimitiveComponent.GetCollisionObjectType` _array_element) "ECC_GameTraceChannel2")
      (`parent.ReceiveActorBeginOverlap` OtherActor))))

(event `self.ReceiveHit`
  (params (MyComp :type "PrimitiveComponent Object Reference") (Other :type "Actor Object Reference") (OtherComp :type "PrimitiveComponent Object Reference") (bSelfMoved :type Boolean) (HitLocation :type "Vector Structure") (HitNormal :type "Vector Structure") (NormalImpulse :type "Vector Structure") (Hit :type "HitResult Structure (by ref)"))
  (`PrimitiveComponent.SetCollisionEnabled` (`self.ActivatedCollision`) "QueryOnly"))

(fn `UserConstructionScript`
  (`parent.UserConstructionScript`)
  (`PrimitiveComponent.SetCollisionEnabled` (`self.ActivatedCollision`) "NoCollision"))