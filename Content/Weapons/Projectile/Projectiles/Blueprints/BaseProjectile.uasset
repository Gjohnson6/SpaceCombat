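; Base projectile Blueprint for weapons that damages the actor it overlaps and then destroys itself.
; On overlap it ignores its owner and any child actors, a temporary fix against hitting weapons, then applies damage credited to its instigator's controller.
; SetDamage sets the damage amount, while SetParent stores a parent reference that the overlap logic does not use.
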(event `self.ReceiveActorBeginOverlap`
  (params (OtherActor :type "Actor Object Reference"))
  (if (!= OtherActor (`self.GetOwner`))
    (if (not (`self.IsChildActor` OtherActor)) :!pinned true
      (`GameplayStatics.ApplyDamage` OtherActor (`self.Damage`) (`self.GetInstigatorController`))
      (`self.K2_DestroyActor`) ; Destroy projectile on impact
    )))

(event `Set Parent`
  (params (Parent :type "Pawn Object Reference"))
  (set `self.Parent` Parent))

(event `self.ReceiveHit`
  (params (MyComp :type "PrimitiveComponent Object Reference") (Other :type "Actor Object Reference") (OtherComp :type "PrimitiveComponent Object Reference") (bSelfMoved :type Boolean) (HitLocation :type "Vector Structure") (HitNormal :type "Vector Structure") (NormalImpulse :type "Vector Structure") (Hit :type "HitResult Structure (by ref)")))

(fn `SetDamage`
  (params (NewDamage :type "Float (double-precision)"))
  (set `self.Damage` NewDamage))

(fn `UserConstructionScript`)