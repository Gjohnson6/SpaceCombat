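; Base homing projectile that explodes for radial falloff damage and can steer toward a target component.
; SetHomingTarget passes that component to the projectile movement component.
; Any hit destroys the actor, and the Destroyed event applies the area damage and spawns an enlarged explosion effect, so any destruction detonates it.
; Construction calls SetDamage with zero; debug spheres for the damage radii are left unconnected.
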(event `self.ReceiveHit`
  (params (MyComp :type "PrimitiveComponent Object Reference") (Other :type "Actor Object Reference") (OtherComp :type "PrimitiveComponent Object Reference") (bSelfMoved :type Boolean) (HitLocation :type "Vector Structure") (HitNormal :type "Vector Structure") (NormalImpulse :type "Vector Structure") (Hit :type "HitResult Structure (by ref)"))
  (`self.K2_DestroyActor`))

(event `self.ReceiveDestroyed`
  (`GameplayStatics.ApplyRadialDamageWithFalloff` :`BaseDamage` (`self.BaseDamage`) :`MinimumDamage` (`self.MinDamage`) :`Origin` (`self.K2_GetActorLocation`) :`DamageInnerRadius` (`self.InnerRadius`) :`DamageOuterRadius` (`self.OuterRadius`) :`DamageFalloff` (`self.Falloff`) :`DamageCauser` (`self.Parent`) :`DamagePreventionChannel` "ECC_WorldDynamic")
  (bind _returnvalue (`GameplayStatics.SpawnEmitterAtLocation` "/Game/StarterContent/Particles/P_Explosion.P_Explosion" (`self.K2_GetActorLocation`)))
  (`SceneComponent.SetWorldScale3D` _returnvalue (5.0 5.0 5.0)))

(event `SetHomingTarget`
  (params (HomingTargetComponent :type "SceneComponent Object Reference"))
  (set `ProjectileMovementComponent.HomingTargetComponent` HomingTargetComponent (`self.ProjectileMovement`)))

(fn `UserConstructionScript`
  (`parent.UserConstructionScript`)
  (`self.SetDamage` 0.0))